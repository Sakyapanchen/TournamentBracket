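; BP_TournamentGameInstance is a game instance that holds experimental VaRest code for reading tournament data from a remote JSON index.
; Init is empty; the response callback stores the JSON object and prints the field names of each "tournaments" entry.
; The URL call bound to that callback is disconnected, as are test snippets for image download, timestamp parsing and request construction.
; A second custom event stores a request and sets its binary content.
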(event `self.ReceiveInit`)

(event `CustomEventdfd`
  (params (Request :type "VaRestRequestJSON Object Reference"))
  (bind _output_get (set `self.Request` Request))
  (`VaRestRequestJSON.SetBinaryRequestContent` _output_get (`|MakeArray` 0 :!type "Byte")))

(event `CustomEvent_0`
  (params (Request :type "VaRestRequestJSON Object Reference"))
  (bind _returnvalue (`VaRestRequestJSON.GetResponseObject` Request))
  (bind _output_get (set `self.ResponceObject` _returnvalue))
  (for _array_element (`VaRestJsonObject.GetArrayField` _output_get "tournaments")
    (bind _returnvalue_2 (`VaRestJsonValue.AsObject` _array_element))
    (for _array_element_2 (`VaRestJsonObject.GetFieldNames` _returnvalue_2)
      (`KismetSystemLibrary.PrintString` _array_element_2 true true (struct :`R` 1.0 :`G` 0.872163 :`A` 1.0) 99.0))))